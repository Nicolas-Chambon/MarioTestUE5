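; Boite is a box actor that spawns a Piece actor the first time its Box component is overlapped.
; On BeginPlay it stores and prints a spawn point at a fixed offset from its own location.
; A DoN gate limits the overlap to one trigger, which prints a "destroyed box" message in French and spawns the Piece there.
; The DestroyActor call is disconnected, so the box itself remains.
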(event OnComponentBeginOverlap(Box)
  (params (OverlappedComponent :type Primitive%20Component%20Object%20Reference) (OtherActor :type Actor%20Object%20Reference) (OtherComp :type Primitive%20Component%20Object%20Reference) (OtherBodyIndex :type Integer) (bFromSweep :type Boolean) (SweepResult :type Hit%20Result%20Structure%20%28by%20ref%29))
  (Utilities|FlowControl|DoN 1
    (:Exit
      (Development|PrintString "Boite détuite" true true "(R=0.546875,G=0.463519,B=0.002848,A=1.000000)" 5.0)
      (Game|SpawnActorfromClass "/Game/Blueprints/Piece.Piece_C" (Math|Transform|MakeTransform (Variables|Default|GetlocationChange) "0,0.000000, 0" "1.000000,1.000000,1.000000") "AlwaysSpawn" 0 0))))

(event EventBeginPlay
  (bind _output_get (Variables|Default|SetlocationChange (Transformation|GetActorLocation)))
  (bind _output_get_2 (Variables|Default|SetlocationChange (+ (Math|Vector|MakeVector 3e+01 0.0 1.4e+02) _output_get)))
  (Development|PrintString (Utilities|String|ToString(Vector) _output_get_2) true true "(R=0.000000,G=0.660000,B=1.000000,A=1.000000)" 1e+02))

(fn ConstructionScript)

(fn NewFunction0)